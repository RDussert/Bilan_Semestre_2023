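; Parent Blueprint for key card items that can be taken and dropped.
; Take teleports the card to the world origin and disables collision on its box and two cube components, rather than destroying it.
; Drop moves the passed-in held object to the CardDropPosition location and restores collision on this card's components.
; Nodes that would finish the associated quest exist but are unconnected and never run.
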(event EventBeginPlay)

(event Collision|EventActorBeginOverlap
  (params (OtherActor :type Actor%20Object%20Reference)))

(event EventTick
  (params (DeltaSeconds :type Float%20%28single-precision%29)))

(event EventTake
  (Transformation|SetActorLocation "0, 0, 0" false false)
  (Collision|SetCollisionEnabled (Variables|Default|GetBox) "NoCollision")
  (Collision|SetCollisionEnabled (Variables|Default|GetCube) "NoCollision")
  (Collision|SetCollisionEnabled (Variables|Default|GetCube1) "NoCollision"))

(event EventDrop
  (params (ObjectInPlayerHand :type Actor%20Object%20Reference))
  (Transformation|SetActorLocation ObjectInPlayerHand (Transformation|GetActorLocation (Variables|Default|GetCardDropPosition)) false false)
  (Collision|SetCollisionEnabled (Variables|Default|GetBox) "QueryAndPhysics")
  (Collision|SetCollisionEnabled (Variables|Default|GetCube) "QueryAndPhysics")
  (Collision|SetCollisionEnabled (Variables|Default|GetCube1) "QueryAndPhysics"))

(fn ConstructionScript)