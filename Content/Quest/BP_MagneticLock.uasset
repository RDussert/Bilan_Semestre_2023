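; BP_MagneticLock is a key card lock that opens a door when the player brings the right card.
; When a BP_ThirdPersonCharacter enters the Box trigger, its ObjectInHand is stored and passed to KeyCardIn.
; If that object matches TrueCard, KeyCardIn switches the red light off and the green on, then snaps the DoorOpen actor to a fixed open rotation.
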(event OnComponentBeginOverlap(Box)
  (params (OverlappedComponent :type Primitive%20Component%20Object%20Reference) (OtherActor :type Actor%20Object%20Reference) (OtherComp :type Primitive%20Component%20Object%20Reference) (OtherBodyIndex :type Integer) (bFromSweep :type Boolean) (SweepResult :type Hit%20Result%20Structure%20%28by%20ref%29))
  (bind _asbp_third_person_character (Utilities|Casting|CastToBP_ThirdPersonCharacter OtherActor))
  (Utilities|IsValid (Variables|/Game/ThirdPerson/Blueprints/BP_ThirdPersonCharacter.BP_ThirdPersonCharacter_C|GetObjectInHand _asbp_third_person_character)
    (:Is%20Valid
      (bind _output_get (Variables|Default|SetCartInserted (Variables|/Game/ThirdPerson/Blueprints/BP_ThirdPersonCharacter.BP_ThirdPersonCharacter_C|GetObjectInHand _asbp_third_person_character)))
      (CallFunction|KeyCardin _output_get))))

(event EventBeginPlay)

(event Collision|EventActorBeginOverlap
  (params (OtherActor :type Actor%20Object%20Reference)))

(event EventTick
  (params (DeltaSeconds :type Float%20%28single-precision%29)))

(fn ConstructionScript)

(fn KeyCardin
  (params (Cart%20Inserted :type Actor%20Object%20Reference))
  (if (== Cart%20Inserted (Variables|Default|GetTrueCard))
    (Rendering|Components|Light|SetIntensity (Variables|/Game/Quest/BP_GreenLight.BP_GreenLight_C|GetPointLight (Variables|Default|GetGreenLight)) 5e+03)
    (Rendering|Components|Light|SetIntensity (Variables|/Game/Quest/BP_RedLight.BP_RedLight_C|GetPointLight (Variables|Default|GetRedLight)) 0.0)
    (Transformation|SetActorRotation (Variables|Default|GetDoorOpen) "0.000000,90.000000,0.000000" true)))