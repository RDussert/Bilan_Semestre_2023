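; Quest actor that tracks task completion and advances the player's quest log.
; On BeginPlay it casts the player to BP_ThirdPersonCharacter and caches its QuestLog after a short delay.
; ProgressionQuest sets IsFinished, which gates TaskFinished: that event marks the current Tasks entry true, increments and prints the LigneQuest index, then calls NextTask on the log.
; IsFinished is never reset here.
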(event Custom|TaskFinished
  (bind _output_get (Variables|Default|SetTasks (Variables|Default|GetTasks)))
  (if (Variables|Default|GetIsFinished)
    (Utilities|Array|SetArrayElem _output_get (Variables|Default|GetLigneQuest) true)
    (bind _result (Math|Integer|IncrementInt (Variables|Default|GetLigneQuest))
      (:%20%20
        (bind _output_get_2 (Variables|Default|SetLigneQuest _result))
        (Development|PrintString (Utilities|String|ToString(Integer) _output_get_2))
        (Default|NextTask (Variables|Default|GetQuest%20Log))))))

(event Collision|EventActorBeginOverlap
  (params (OtherActor :type Actor%20Object%20Reference)))

(event EventTick
  (params (DeltaSeconds :type Float%20%28single-precision%29)))

(event EventBeginPlay
  (bind _asbp_third_person_character (Utilities|Casting|CastToBP_ThirdPersonCharacter (Game|GetPlayerCharacter 0)))
  (Utilities|FlowControl|Delay 0.1)
  (Variables|Default|SetQuest%20Log (Variables|/Game/ThirdPerson/Blueprints/BP_ThirdPersonCharacter.BP_ThirdPersonCharacter_C|GetQuestLog _asbp_third_person_character)))

(fn ConstructionScript)

(fn ProgressionQuest
  (Variables|Default|SetIsFinished true))